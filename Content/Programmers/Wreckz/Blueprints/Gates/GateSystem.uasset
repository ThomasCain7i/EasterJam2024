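; Gate actor that snaps its two gate pieces to fixed rotations when its box trigger is overlapped and the player holds the matching egg.
; BeginPlay caches the first-person character.
; The overlap walks an if-chain pairing five egg flags with Gate1–5 checks, without checking which actor overlapped.
; Every successful branch applies the same rotations to Gate1 and Gate2, then plays a gate slam sound.
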(event OnComponentBeginOverlap(Box)
  (params (OverlappedComponent :type Primitive%20Component%20Object%20Reference) (OtherActor :type Actor%20Object%20Reference) (OtherComp :type Primitive%20Component%20Object%20Reference) (OtherBodyIndex :type Integer) (bFromSweep :type Boolean) (SweepResult :type Hit%20Result%20Structure%20%28by%20ref%29))
  (if (and (Variables|/Game/FirstPerson/Blueprints/BP_FirstPersonCharacter.BP_FirstPersonCharacter_C|GetHasEgg1? (stale EventBeginPlay _asbp_first_person_character)) (Variables|Default|GetGate%201))
    (Transformation|SetRelativeRotation (Variables|Default|GetGate1) "0, 0, 0" false false)
    (Transformation|SetRelativeRotation (Variables|Default|GetGate2) "0.000000,180.000000,0.000000" false false)
    (Audio|PlaySound2D "/Game/Audio/GateSlam_Cue.GateSlam_Cue" 1.0 1.0 0.0 0 0 :!label _label)
    (elif (and (Variables|/Game/FirstPerson/Blueprints/BP_FirstPersonCharacter.BP_FirstPersonCharacter_C|GetHasEgg2? (stale EventBeginPlay _asbp_first_person_character)) (Variables|Default|GetGate%202))
      (Transformation|SetRelativeRotation (Variables|Default|GetGate1) "0, 0, 0" false false)
      (Transformation|SetRelativeRotation (Variables|Default|GetGate2) "0.000000,180.000000,0.000000" false false)
      (goto _label)
      (elif (and (Variables|/Game/FirstPerson/Blueprints/BP_FirstPersonCharacter.BP_FirstPersonCharacter_C|GetHasEgg3? (stale EventBeginPlay _asbp_first_person_character)) (Variables|Default|GetGate%203))
        (Transformation|SetRelativeRotation (Variables|Default|GetGate1) "0, 0, 0" false false)
        (Transformation|SetRelativeRotation (Variables|Default|GetGate2) "0.000000,180.000000,0.000000" false false)
        (goto _label)
        (elif (and (Variables|/Game/FirstPerson/Blueprints/BP_FirstPersonCharacter.BP_FirstPersonCharacter_C|GetHasEgg4? (stale EventBeginPlay _asbp_first_person_character)) (Variables|Default|GetGate%204))
          (Transformation|SetRelativeRotation (Variables|Default|GetGate1) "0, 0, 0" false false)
          (Transformation|SetRelativeRotation (Variables|Default|GetGate2) "0.000000,180.000000,0.000000" false false)
          (goto _label)
          (elif (and (Variables|/Game/FirstPerson/Blueprints/BP_FirstPersonCharacter.BP_FirstPersonCharacter_C|GetHasEgg5? (stale EventBeginPlay _asbp_first_person_character)) (Variables|Default|GetGate%205))
            (Transformation|SetRelativeRotation (Variables|Default|GetGate1) "0, 0, 0" false false)
            (Transformation|SetRelativeRotation (Variables|Default|GetGate2) "0.000000,180.000000,0.000000" false false)
            (goto _label)))))))

(event EventBeginPlay
  (bind _asbp_first_person_character (Utilities|Casting|CastToBP_FirstPersonCharacter (Game|GetPlayerCharacter 0))))

(fn ConstructionScript)