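; Enemy rabbit AI that patrols a looping list of patrol points, chases the first-person player on sight, and attacks on contact.
; PawnSensing triggers a snarl and chase, while Tick resumes patrol once sight lapses.
; Box overlap applies damage once, then restarts the route, with attacks re-arming as patrol advances.
; Phase events escalate speed, sight and patrol pacing, culminating in TheHunt, which sets the player's Forcekill flag and pursues them, retrying failed moves.
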(event OnSeePawn(PawnSensing)
  (params (Pawn :type Pawn%20Object%20Reference))
  (bind _asbp_first_person_character (Utilities|Casting|CastToBP_FirstPersonCharacter Pawn))
  (Utilities|FlowControl|Sequence
    (:then_0
      (if (not (Variables|Default|GetHasAttacked?))
        (CallFunction|Playsound "/Game/Audio/Cues/Rabbit/SC_RabbitSnarl.SC_RabbitSnarl")
        (Variables|Default|SetSeeEnemy? true)
        (AI|AIMoveTo self "0, 0, 0" _asbp_first_person_character (Variables|Default|GetAcceptance%20Radius) false
          (:OnSuccess
            (Utilities|FlowControl|DoOnce false)))))
    (:then_1
      (Utilities|FlowControl|RetriggerableDelay 0.6)
      (Variables|Default|SetSeeEnemy? false))))

(event OnComponentBeginOverlap(Box)
  (params (OverlappedComponent :type Primitive%20Component%20Object%20Reference) (OtherActor :type Actor%20Object%20Reference) (OtherComp :type Primitive%20Component%20Object%20Reference) (OtherBodyIndex :type Integer) (bFromSweep :type Boolean) (SweepResult :type Hit%20Result%20Structure%20%28by%20ref%29))
  (if (not (Variables|Default|GetHasAttacked?))
    (Game|Damage|ApplyDamage OtherActor (Variables|Default|GetDamage) 0 0)
    (CallFunction|Playsound "/Game/Audio/Cues/Rabbit/SC_RabbitGrowl.SC_RabbitGrowl")
    (Variables|Default|SetHasAttacked? true)
    (Variables|Default|SetPatrol%20Point%20Index 0)
    (CallFunction|Patrol)))

(event Custom|Patrol
  (AI|AIMoveTo self "0, 0, 0" (Utilities|Array|Get(acopy) (Variables|Default|GetPatrol%20Point) (Variables|Default|GetPatrol%20Point%20Index)) 5.0 false
    (:OnSuccess
      (Utilities|FlowControl|Delay (Variables|Default|GetWaitTime))
      (if (>= (Variables|Default|GetPatrol%20Point%20Index) (- (Utilities|Array|Length (Variables|Default|GetPatrol%20Point)) 1))
        (Variables|Default|SetPatrol%20Point%20Index 0)
        (else
          (Variables|Default|SetHasAttacked? false)
          (Math|Integer|IncrementInt (Variables|Default|GetPatrol%20Point%20Index)
            (:%20%20
              _))))
      (CallFunction|Patrol))))

(event Custom|The%20Hunt
  (Variables|/Game/FirstPerson/Blueprints/BP_FirstPersonCharacter.BP_FirstPersonCharacter_C|SetForcekill (Variables|Default|GetPlayer%20REF) true)
  (Variables|/Script/Engine.CharacterMovementComponent|SetMaxWalkSpeed (Variables|Character|GetCharacterMovement) 1.2e+03)
  (Variables|Default|SetDamage 3.0)
  (Variables|Default|SetWaitTime 0.0)
  (Audio|PlaySound2D "/Game/Audio/Cues/Church/Bellstrike_Cue.Bellstrike_Cue" 1.0 1.0 0.0 0 0)
  (AI|AIMoveTo self "0, 0, 0" (Variables|Default|GetPlayer%20REF) 5.0 false :!label _label
    (:OnFail
      (Utilities|FlowControl|Delay 0.1)
      (goto _label))))

(event Custom|Phase%201
  (Variables|/Script/Engine.CharacterMovementComponent|SetMaxWalkSpeed (Variables|Character|GetCharacterMovement) 6e+02)
  (Variables|Default|SetWaitTime 2.0))

(event Custom|Phase%202
  (Variables|/Script/AIModule.PawnSensingComponent|SetSightRadius (Variables|Default|GetPawnSensing) 3e+03))

(event Custom|Phase%203
  (Variables|/Script/Engine.CharacterMovementComponent|SetMaxWalkSpeed (Variables|Character|GetCharacterMovement) 7e+02)
  (Variables|/Script/AIModule.PawnSensingComponent|SetSightRadius (Variables|Default|GetPawnSensing) 3.5e+03)
  (Variables|Default|SetWaitTime 1.5))

(event Custom|Phase%204
  (Variables|/Script/Engine.CharacterMovementComponent|SetMaxWalkSpeed (Variables|Character|GetCharacterMovement) 8e+02)
  (Variables|/Script/AIModule.PawnSensingComponent|SetSightRadius (Variables|Default|GetPawnSensing) 4e+03)
  (Variables|Default|SetWaitTime 1.0))

(event EventBeginPlay
  (CallFunction|Patrol)
  (bind _foundwidgets (Widget|GetAllWidgetsOfClass "/Game/Programmers/Wreckz/Widgets/HUD.HUD_C" true))
  (Variables|Default|SetHUD%20REF (Utilities|Array|Get(acopy) _foundwidgets))
  (bind _asbp_first_person_character (Utilities|Casting|CastToBP_FirstPersonCharacter (Game|GetPlayerCharacter 0)))
  (Variables|Default|SetPlayer%20REF _asbp_first_person_character))

(event EventTick
  (params (DeltaSeconds :type Float%20%28single-precision%29))
  (if (not (Variables|Default|GetSeeEnemy?))
    (Utilities|FlowControl|Delay 0.4)
    (if (not (Variables|Default|GetSeeEnemy?))
      (CallFunction|Patrol))))

(fn ConstructionScript)

(fn PatroltoPoint)

(fn Playsound
  (params (NewSound :type Sound%20Base%20Object%20Reference))
  (bind _rabbit (Variables|Default|GetRabbit))
  (Audio|Components|Audio|SetSound _rabbit NewSound)
  (Audio|Components|Audio|Play _rabbit 0.0))