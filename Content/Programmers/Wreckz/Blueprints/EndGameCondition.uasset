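; EndGameCondition is a trigger actor that ends the game when its box is overlapped while the player has exactly five eggs.
; It caches the first-person character on BeginPlay and reads its egg count on overlap, without checking which actor entered.
; On success it re-adds the existing HUD to the viewport, switches it to index 2, enables UI-only input with a cursor and pauses the game.
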(event OnComponentBeginOverlap(Box)
  (params (OverlappedComponent :type Primitive%20Component%20Object%20Reference) (OtherActor :type Actor%20Object%20Reference) (OtherComp :type Primitive%20Component%20Object%20Reference) (OtherBodyIndex :type Integer) (bFromSweep :type Boolean) (SweepResult :type Hit%20Result%20Structure%20%28by%20ref%29))
  (bind _returnvalue (Game|GetPlayerController 0))
  (if (== (Variables|/Game/FirstPerson/Blueprints/BP_FirstPersonCharacter.BP_FirstPersonCharacter_C|GetNumberOfEggs (stale EventBeginPlay _asbp_first_person_character)) 5)
    (bind _foundwidgets (Widget|GetAllWidgetsOfClass "/Game/Programmers/Wreckz/Widgets/HUD.HUD_C" true))
    (Widget|RemovefromParent (Utilities|Array|Get(acopy) _foundwidgets))
    (UserInterface|Viewport|AddtoViewport (Utilities|Array|Get(acopy) _foundwidgets) 0)
    (Class|WidgetSwitcher|SetActiveWidgetIndex (Variables|/Game/Programmers/Wreckz/Widgets/HUD.HUD_C|GetHUDWidgetSwitcher (Utilities|Array|Get(acopy) _foundwidgets)) 2)
    (Input|SetInputModeUIOnly _returnvalue 0 "DoNotLock" false)
    (Variables|/Script/Engine.PlayerController|SetbShowMouseCursor _returnvalue true)
    (Game|SetGamePaused true)))

(event EventBeginPlay
  (bind _asbp_first_person_character (Utilities|Casting|CastToBP_FirstPersonCharacter (Game|GetPlayerCharacter 0))))

(fn ConstructionScript)