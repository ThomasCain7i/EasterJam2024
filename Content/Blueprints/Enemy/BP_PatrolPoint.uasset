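; BP_PatrolPoint is an enemy patrol point that registers itself with the game instance.
; On BeginPlay it waits briefly, then casts and caches BP_GameInstance and passes itself to AddPatrolPoint.
; It holds no patrol logic of its own, and its construction script is empty.
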(event Custom|Setup
  (bind _asbp_game_instance (Utilities|Casting|CastToBP_GameInstance (Game|GetGameInstance)))
  (Variables|Default|SetAs%20BP%20Game%20Instance _asbp_game_instance))

(event Custom|SubscribeToGameInstance
  (Default|AddPatrolPoint (Variables|Default|GetAs%20BP%20Game%20Instance) self))

(event EventBeginPlay
  (Utilities|FlowControl|Delay 0.1)
  (CallFunction|Setup)
  (CallFunction|SubscribetoGameInstance))

(fn ConstructionScript)