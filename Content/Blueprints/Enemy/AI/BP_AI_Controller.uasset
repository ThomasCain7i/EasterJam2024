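; Enemy AI controller that runs the BT_Enemy behavior tree and supplies random patrol destinations.
; After a short delay on BeginPlay, it caches the game instance and copies its shared patrol points into a local list before starting the tree.
; The SendPatrolPoint event picks a random patrol point, finds a navigable location close to it and writes that to the TargetLocation blackboard key.
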(event Custom|Setup
  (bind _asbp_game_instance (Utilities|Casting|CastToBP_GameInstance (Game|GetGameInstance)))
  (Variables|Default|SetAs%20BP%20Game%20Instance _asbp_game_instance))

(event Custom|GetControlPoints
  (for _array_element (Variables|/Game/FirstPerson/Blueprints/BP_GameInstance.BP_GameInstance_C|GetPatrolPoints (Variables|Default|GetAs%20BP%20Game%20Instance))
    (Utilities|Array|AddUnique (Variables|Default|GetPatrolPoints) _array_element)))

(event EventSendPatrolPoint
  (bind _randomlocation (Class|NavigationSystemV1|GetRandomLocationinNavigableRadius (Transformation|GetWorldLocation (Variables|/Game/Blueprints/Enemy/BP_PatrolPoint.BP_PatrolPoint_C|GetDefaultSceneRoot (.OutItem (Utilities|Array|Random (Variables|Default|GetPatrolPoints))))) 2e+01 0 0))
  (AI|Components|Blackboard|SetValueasVector (AI|GetBlackboard self) (Utilities|Name|MakeLiteralName "TargetLocation") _randomlocation))

(event EventBeginPlay
  (Utilities|FlowControl|Delay 0.3)
  (CallFunction|Setup)
  (CallFunction|GetControlPoints)
  (AI|RunBehaviorTree "/Game/Blueprints/Enemy/AI/BT_Enemy.BT_Enemy"))

(fn ConstructionScript)