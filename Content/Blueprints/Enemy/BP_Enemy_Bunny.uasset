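; Bunny enemy Blueprint that tells its AI whether it has seen the player.
; When PawnSensing spots the first-person character, it sets the bHasSeenPlayer Blackboard key and starts an eight-second timer.
; When that timer fires, StopChasing clears the key and invalidates the timer handle.
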(event OnSeePawn(PawnSensing)
  (params (Pawn :type Pawn%20Object%20Reference))
  (Utilities|Casting|CastToBP_FirstPersonCharacter Pawn)
  (AI|Components|Blackboard|SetValueasBool (AI|GetBlackboard (AI|GetAIController self)) (Utilities|Name|MakeLiteralName "bHasSeenPlayer") true)
  (bind _returnvalue (Utilities|Time|SetTimerbyEvent (delegate Custom|StopChasing) 8.0))
  (Variables|Default|SetLookTimer _returnvalue))

(event Custom|StopChasing
  (AI|Components|Blackboard|SetValueasBool (AI|GetBlackboard (AI|GetAIController self)) (Utilities|Name|MakeLiteralName "bHasSeenPlayer") false)
  (Utilities|Time|ClearandInvalidateTimerbyHandle (Variables|Default|GetLookTimer)))

(fn ConstructionScript)