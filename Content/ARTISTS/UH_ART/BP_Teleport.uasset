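; BP_Teleport is a teleport effect actor that plays a cultist cast-escape animation once on BeginPlay.
; It creates a dynamic cultist material and adds a Niagara system bound to the skeletal mesh.
; Each tick, TeleCurve sampled at the animation position drives the material's Phase parameter and is printed for debugging.
; Once the curve value exceeds one, the Niagara spawn rate is set to zero.
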(event EventBeginPlay
  (bind _skeletalmesh (Variables|Default|GetSkeletalMesh))
  (Components|Animation|PlayAnimation _skeletalmesh "/Game/ARTISTS/UH_ART/Cultist7_Anim_root_1_CastEscape.Cultist7_Anim_root_1_CastEscape" false)
  (bind _returnvalue (Rendering|Material|CreateDynamicMaterialInstance _skeletalmesh 0 "/Game/ARTISTS/UH_ART/MI_Cultist.MI_Cultist" "None" :!class /Script/Engine.PrimitiveComponent))
  (bind _returnvalue_2 (AddComponent|AddNiagaraComponent false))
  (Class|NiagaraFunctionLibrary|OverrideSystemUserVariableSkeletalMeshComponent _returnvalue_2 "" _skeletalmesh))

(event Collision|EventActorBeginOverlap
  (params (OtherActor :type Actor%20Object%20Reference)))

(event EventTick
  (params (DeltaSeconds :type Float%20%28single-precision%29))
  (bind _skeletalmesh (Variables|Default|GetSkeletalMesh))
  (bind _telecurve (Variables|Default|GetTeleCurve))
  (bind _returnvalue (Class|SkeletalMeshComponent|GetPosition _skeletalmesh))
  (bind _returnvalue_2 (Math|Curves|GetFloatValue _telecurve _returnvalue))
  (Development|PrintText (Utilities|Text|ToText(Float) _returnvalue_2 "HalfToEven"))
  (Rendering|Material|SetScalarParameterValue (stale EventBeginPlay _returnvalue) "Phase" _returnvalue_2 :!class /Script/Engine.MaterialInstanceDynamic)
  (if (> _returnvalue_2 1.0)
    (Niagara|SetNiagaraVariable(Float) (stale EventBeginPlay _returnvalue_2) "Spawnrate" 0.0)))

(fn ConstructionScript)