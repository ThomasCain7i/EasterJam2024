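; BP_Cultist is a cultist Blueprint that plays a material-driven teleport effect on its skeletal mesh.
; BeginPlay caches the ABP_Cultist anim instance and creates a dynamic instance of MI_Cultist.
; The Teleport event sets the anim instance's Teleport flag, which Tick polls to start the Gradient timeline through a DoOnce.
; The timeline drives the material's Phase parameter; the DoOnce never resets, and the actor itself is not moved.
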(event Custom|Teleport
  (Variables|/Game/ARTISTS/UH_ART/ABP_Cultist.ABP_Cultist_C|SetTeleport (Variables|Default|GetAs%20ABP%20Cultist) true))

(event EventBeginPlay
  (bind _skeletalmesh (Variables|Default|GetSkeletalMesh))
  ;[1 0 0.09863] Comment
  (bind _asabp_cultist (Utilities|Casting|CastToABP_Cultist (Components|SkeletalMesh|GetAnimInstance _skeletalmesh)))
  (Variables|Default|SetAs%20ABP%20Cultist _asabp_cultist)
  (bind _returnvalue (Rendering|Material|CreateDynamicMaterialInstance _skeletalmesh 0 "/Game/ARTISTS/UH_ART/MI_Cultist.MI_Cultist" "None" :!class /Script/Engine.PrimitiveComponent))
  (Variables|Default|SetMaterial%20Dynamic _returnvalue))

(event EventTick
  (params (DeltaSeconds :type Float%20%28single-precision%29))
  ;[1 0 0.5533] Payload
  (if (Variables|/Game/ARTISTS/UH_ART/ABP_Cultist.ABP_Cultist_C|GetTeleport (Variables|Default|GetAs%20ABP%20Cultist))
    (Utilities|FlowControl|DoOnce false
      (:Completed
        (bind _newtrack_0 (Timeline|Gradient Play)
          (:Update
            (Rendering|Material|SetScalarParameterValue (Variables|Default|GetMaterial%20Dynamic) "Phase" _newtrack_0 :!class /Script/Engine.MaterialInstanceDynamic)))))))

(fn ConstructionScript)