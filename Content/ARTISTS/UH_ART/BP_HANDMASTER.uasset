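; BP_HANDMASTER drives a hand skeletal mesh through its ABP_HANDMASTER animation Blueprint and also references a Control Rig.
; BeginPlay casts and caches the mesh's anim instance, then Tick copies the Speed and Idle variables into it every frame.
; Tick also prints the local-space position of the rig's root_ctrl control, apparently as debug output.
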(event EventBeginPlay
  (bind _asabp_handmaster (Utilities|Casting|CastToABP_HANDMASTER (Components|SkeletalMesh|GetAnimInstance (Variables|Default|GetSkeletalMesh))))
  (Variables|Default|SetAnimInstance _asabp_handmaster))

(event EventTick
  (params (DeltaSeconds :type Float%20%28single-precision%29))
  (bind _animinstance (Variables|Default|GetAnimInstance))
  (Variables|/Game/ARTISTS/UH_ART/ABP_HANDMASTER.ABP_HANDMASTER_C|SetSpeed _animinstance (Variables|Default|GetSpeed))
  (Variables|/Game/ARTISTS/UH_ART/ABP_HANDMASTER.ABP_HANDMASTER_C|SetIdle _animinstance (Variables|Default|GetIdle))
  (Development|PrintText (Utilities|Text|ToText(String) (Class|ControlRigComponent|GetControlPosition (Variables|Default|GetControlRig) "root_ctrl" "LocalSpace"))))

(fn ConstructionScript)